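; BP_DimensionChecker_3406x4861 is a house-design decal actor that projects a furniture placement image, apparently as a size guide.
; The construction script creates a dynamic material instance on the decal and feeds it the image, base color and emission strength.
; It also sets the decal's X scale to the default height for full coverage, or to the floor height otherwise.
; BeginPlay applies the VisibleInGame setting to the decal's visibility.
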(event `self.ReceiveBeginPlay`
  (`SceneComponent.SetVisibility` (`self.Decal`) (`self.VisibleInGame`) false))

(fn `UserConstructionScript`
  (bind _decal (`self.Decal`))
  (bind (_relativescale3d_x _relativescale3d_y _relativescale3d_z) (`KismetMathLibrary.BreakVector` (`SceneComponent.RelativeScale3D` _decal)))
  (`|ExecutionSequence`
    (:`then_0`
      (bind _returnvalue (`DecalComponent.CreateDynamicMaterialInstance` (`self.Decal`)))
      (`MaterialInstanceDynamic.SetTextureParameterValue` _returnvalue "Texture" (`self.FurniturePlacementImage`))
      (`MaterialInstanceDynamic.SetVectorParameterValue` _returnvalue "Base Color" (`self.Color`))
      (`MaterialInstanceDynamic.SetScalarParameterValue` _returnvalue "Emission Strength" (`self.Emission Strength`)))
    (:`then_1`
      (if (`self.Full Coverage`)
        (`SceneComponent.SetRelativeScale3D` _decal (`KismetMathLibrary.MakeVector` (`self.Default Height`) _relativescale3d_y _relativescale3d_z))
        (else
          (`SceneComponent.SetRelativeScale3D` _decal (`KismetMathLibrary.MakeVector` (`self.Floor Height`) _relativescale3d_y _relativescale3d_z)))))))