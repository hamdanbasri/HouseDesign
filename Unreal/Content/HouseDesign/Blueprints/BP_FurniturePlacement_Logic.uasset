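; Furniture placement marker for house design that shows a configurable image on the SMDimensionChecker component.
; The construction script creates a dynamic instance of a furniture decal material and feeds it the actor's placement image, color and emission strength, so each placement gets its own look.
; On BeginPlay, the VisibleInGame flag decides whether the component shows during play, without propagating to its children.
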(event `self.ReceiveBeginPlay`
  (`SceneComponent.SetVisibility` (`self.SM_DimensionChecker`) (`self.VisibleInGame`) false))

(fn `UserConstructionScript`
  (bind _returnvalue (`PrimitiveComponent.CreateDynamicMaterialInstance` (`self.SM_DimensionChecker`) 0 "/Game/Materials/MaterialInstance/Decal/MI_Decal_Furniture_TypeG.MI_Decal_Furniture_TypeG" "None"))
  (`MaterialInstanceDynamic.SetTextureParameterValue` _returnvalue "Texture" (`self.FurniturePlacementImage`))
  (`MaterialInstanceDynamic.SetVectorParameterValue` _returnvalue "Base Color" (`self.Color`))
  (`MaterialInstanceDynamic.SetScalarParameterValue` _returnvalue "Emission Strength" (`self.Emission Strength`)))