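; BP_Spotlight_Placement is a house-design actor that places a spotlight fixture on the surface above it.
; While HeightAchieved is false, Tick or PlaceinPosition traces 1500 units along the actor's up vector and spawns a movable SpotLight and a mesh actor at the impact point, without checking for a hit.
; The flag then blocks repeats until ResetLocation clears it and resets Holder's relative position.
; Holder and Ring are hidden during play.
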(event `self.ReceiveBeginPlay`
  (`SceneComponent.SetHiddenInGame` (`self.Holder`) true false)
  (`SceneComponent.SetHiddenInGame` (`self.Ring`) true false))

(event `Reset Location`
  ;[0.4637 0.6062 1] Reset
  (`SceneComponent.K2_SetRelativeLocation` (`self.Holder`) (0.0 0.0 15.0) false false)
  (set `self.HeightAchieved` false))

(event `Place in Position`
  (bind (_returnvalue_location _returnvalue_rotation) (`KismetMathLibrary.BreakTransform` (`self.GetTransform`)))
  ;[0.6134 1 0.6421] Place in Position
  (if (not (`self.HeightAchieved`)) :!label _label
    (bind _outhit (`KismetSystemLibrary.LineTraceSingle` :`Start` _returnvalue_location :`End` (+ _returnvalue_location (* (`KismetMathLibrary.GetUpVector` _returnvalue_rotation) 1500.0)) :`TraceChannel` "TraceTypeQuery1" :`bTraceComplex` true :`DrawDebugType` "ForOneFrame"))
    (bind _returnvalue (`KismetMathLibrary.Conv_VectorToTransform` (`.ImpactPoint` (`GameplayStatics.BreakHitResult` _outhit))))
    (bind _returnvalue_2 (`|SpawnActorFromClass` "/Script/Engine.SpotLight" _returnvalue "Undefined" "MultiplyWithRoot" null null))
    (`SceneComponent.SetMobility` (`SpotLight.SpotLightComponent` _returnvalue_2) "Movable")
    (set `self.HeightAchieved` true)
    (bind _returnvalue_3 (`|SpawnActorFromClass` "/Script/Engine.StaticMeshActor" _returnvalue "Undefined" "MultiplyWithRoot" null null))
    (`StaticMeshComponent.SetStaticMesh` (`StaticMeshActor.StaticMeshComponent` _returnvalue_3) (`self.StatMesh`))))

(event `self.ReceiveTick`
  (params (DeltaSeconds :type "Float (single-precision)"))
  ;[0.6134 1 0.6421] Place in Position
  (goto _label))

(fn `UserConstructionScript`)