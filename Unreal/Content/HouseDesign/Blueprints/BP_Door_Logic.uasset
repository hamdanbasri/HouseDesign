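; Clickable door actor that toggles open and closed when its Door_Placeholder is clicked.
; Two timelines play or reverse together: Handle pitches the handle, while Duration swings the whole actor between its BeginPlay yaw and OpeningRotation, using RInterpTo as a timeline-driven blend.
; The construction script points a direction arrow by the sign of OpeningRotation, and BeginPlay shows or hides it via ShowDirectionalArrows.
; Several disconnected leftover nodes never run.
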(event `self.ReceiveBeginPlay`
  (bind (_returnvalue_roll _returnvalue_pitch _returnvalue_yaw) (`KismetMathLibrary.BreakRotator` (`self.K2_GetActorRotation`)))
  (set `self.ClosingRotation` _returnvalue_yaw)
  (`SceneComponent.SetVisibility` (`self.SM_DirectionArrow`) (`self.ShowDirectionalArrows`) false))

(event `self.Door_Placeholder.OnClicked`
  (params (TouchedComponent :type "PrimitiveComponent Object Reference") (ButtonPressed :type "Key Structure"))
  (if (`self.isOpen`)
    (set `self.isOpen` false)
    (`|ExecutionSequence`
      (:`then_0`
        (bind (_direction _y_angle) (`Timeline|Handle` :!via `Reverse` :!label _label)
          (:`Update`
            (`SceneComponent.K2_SetRelativeRotation` (`self.Handle_Placeholder`) (`KismetMathLibrary.MakeRotator` 0.0 _y_angle) false false))))
      (:`then_1`
        (bind (_direction_2 _time) (`Timeline|Duration` :!via `Reverse` :!label _label_2)
          (:`Update`
            (`self.K2_SetActorRotation` (`KismetMathLibrary.RInterpTo` (`KismetMathLibrary.MakeRotator` 0.0 0.0 (`self.ClosingRotation`)) (`KismetMathLibrary.MakeRotator` 0.0 0.0 (`self.OpeningRotation`)) _time 1.0))))))
    (else
      (set `self.isOpen` true)
      (`|ExecutionSequence`
        (:`then_0`
          (goto _label))
        (:`then_1`
          (goto _label_2))))))

(fn `UserConstructionScript`
  (bind _sm_directionarrow (`self.SM_DirectionArrow`))
  (if (>= (`self.OpeningRotation`) 0.0)
    (`SceneComponent.K2_SetRelativeRotation` _sm_directionarrow (`KismetMathLibrary.MakeRotator` 0.0 0.0 90.0) false false)
    (else
      (`SceneComponent.K2_SetRelativeRotation` _sm_directionarrow (`KismetMathLibrary.MakeRotator` 0.0 0.0 -90.0) false false))))