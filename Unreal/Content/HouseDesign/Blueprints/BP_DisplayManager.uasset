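; BP_DisplayManager toggles the visibility of furniture and lighting in the house design scene.
; On BeginPlay it caches all actors tagged "Furniture" and "Lighting".
; The FurnitureDisplay and LightingDisplay events show or hide each group, flipping a state flag and updating a label text.
; The lighting toggle also sets Emission Strength in MPC_Emission, so emissive materials switch with the lights.
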(event `Furniture Display`
  (bind _furnitureactors (`self.FurnitureActors`))
  ;[0 1 0.04795] Furniture Display
  (if (`self.FurnitureDisplay`)
    (for _array_element _furnitureactors
      (`self.SetActorHiddenInGame` _array_element false)
      (set `self.FurnitureDisplay` false)
      (set `self.FurnitureText` "Hide"))
    (else
      (for _array_element_2 _furnitureactors
        (`self.SetActorHiddenInGame` _array_element_2 true)
        (set `self.FurnitureDisplay` true)
        (set `self.FurnitureText` "Show")))))

(event `self.ReceiveBeginPlay`
  (`|ExecutionSequence`
    (:`then_0`
      (bind _outactors (`GameplayStatics.GetAllActorsWithTag` "Furniture"))
      (set `self.FurnitureActors` _outactors))
    (:`then_1`
      (bind _outactors_2 (`GameplayStatics.GetAllActorsWithTag` "Lighting"))
      (set `self.LightingActors` _outactors_2))))

(event `Lighting Display`
  (bind _lightingactors (`self.LightingActors`))
  ;[0 0.7777 1] Lighting Display
  (if (`self.LightingDisplay`)
    (for _array_element _lightingactors
      (`self.SetActorHiddenInGame` _array_element false)
      (set `self.LightingDisplay` false)
      (set `self.LightingText` "Off")
      (`KismetMaterialLibrary.SetScalarParameterValue` "/Game/Materials/MPC_Emission.MPC_Emission" "Emission Strength" 10.0))
    (else
      (for _array_element_2 _lightingactors
        (`self.SetActorHiddenInGame` _array_element_2 true)
        (set `self.LightingDisplay` true)
        (set `self.LightingText` "On")
        (`KismetMaterialLibrary.SetScalarParameterValue` "/Game/Materials/MPC_Emission.MPC_Emission" "Emission Strength" 0.0)))))

(fn `UserConstructionScript`)