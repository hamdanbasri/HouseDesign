(fn `Clear Equipments`
  (`KismetArrayLibrary.Array_Clear` (`self.Spotlight Actors`))
  (`KismetArrayLibrary.Array_Clear` (`self.Switch Actors`)))

(fn `Create Spotlight`
  (bind _returnvalue (`|SpawnActorFromClass` "/Game/HouseDesign/Blueprints/BP_Spotlight_Placement.BP_Spotlight_Placement_C" (`KismetMathLibrary.MakeTransform` (0.0 0.0 0.0)) "Undefined" "MultiplyWithRoot" null null))
  (`KismetArrayLibrary.Array_Add` (`self.Spotlight Actors`) _returnvalue))

(fn `Place Equipments`
  (`|ExecutionSequence`
    (:`then_0`
      (bind _outactors (`GameplayStatics.GetAllActorsOfClass` "/Game/HouseDesign/Blueprints/BP_Spotlight_Placement.BP_Spotlight_Placement_C"))
      (bind _output_get (set `self.Spotlight Actors` _outactors))
      (for _array_element _output_get
        (`/Game/HouseDesign/Blueprints/BP_Spotlight_Placement.Place in Position` _array_element)))
    (:`then_1`
      (bind _outactors_2 (`GameplayStatics.GetAllActorsOfClass` "/Game/HouseDesign/Blueprints/BP_Switch_Placement.BP_Switch_Placement_C"))
      (bind _output_get_2 (set `self.Switch Actors` _outactors_2))
      (for _array_element_2 _output_get_2
        (`/Game/HouseDesign/Blueprints/BP_Switch_Placement.Place in Position` _array_element_2)))))

(fn `Reset Equipments`
  (`|ExecutionSequence`
    (:`then_0`
      (for _array_element (`self.Spotlight Actors`)
        (`/Game/HouseDesign/Blueprints/BP_Spotlight_Placement.Reset Location` _array_element)))
    (:`then_1`
      (for _array_element_2 (`self.Switch Actors`)
        (`/Game/HouseDesign/Blueprints/BP_Switch_Placement.Reset Location` _array_element_2)))))

(fn `UserConstructionScript`)

(fn `WIP | Remove Spotlight`
  (bind _spotlight_actors (`self.Spotlight Actors`))
  (`KismetArrayLibrary.Array_Remove` _spotlight_actors (`KismetArrayLibrary.Array_LastIndex` _spotlight_actors)))