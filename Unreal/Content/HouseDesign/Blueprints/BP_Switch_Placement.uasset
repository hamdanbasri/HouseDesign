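; Switch placement helper that puts a switch mesh onto whatever surface lies in front of it, at a set height.
; The construction script previews SwitchMesh, and BeginPlay hides the holder, arrow and text helpers.
; PlaceinPosition line-traces forward and spawns a separate StaticMeshActor at the impact X/Y and SwitchHeight, using the preview's rotation.
; An IsPlaced flag blocks repeat placement until ResetLocation clears it and re-zeroes the holder, leaving spawned actors untouched.
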(event `self.ReceiveBeginPlay`
  (`SceneComponent.SetHiddenInGame` (`self.Holder`) true false)
  (`SceneComponent.SetHiddenInGame` (`self.Arrow`) true false)
  (`SceneComponent.SetHiddenInGame` (`self.TextRender`) true false))

(event `Reset Location`
  ;[0.4117 0.76 1] Reset
  (`SceneComponent.K2_SetRelativeLocation` (`self.Holder`) (0.0 0.0 0.0) false false)
  (set `self.isPlaced` false))

(event `Place in Position`
  (bind (_returnvalue_location _returnvalue_rotation) (`KismetMathLibrary.BreakTransform` (`self.GetTransform`)))
  ;[0.6735 1 0.6985] Place in Position
  (if (not (`self.isPlaced`))
    (bind _outhit (`KismetSystemLibrary.LineTraceSingle` :`Start` _returnvalue_location :`End` (+ _returnvalue_location (* (`KismetMathLibrary.GetForwardVector` _returnvalue_rotation) 1000.0)) :`TraceChannel` "TraceTypeQuery1" :`bTraceComplex` true :`DrawDebugType` "ForOneFrame"))
    (bind (_bblockinghit _binitialoverlap _time _distance _location _impactpoint) (`GameplayStatics.BreakHitResult` _outhit))
    (bind _returnvalue (`|SpawnActorFromClass` "/Script/Engine.StaticMeshActor" (`KismetMathLibrary.MakeTransform` (`KismetMathLibrary.MakeVector` (.x _impactpoint) (.y _impactpoint) (`self.SwitchHeight`)) (`SceneComponent.K2_GetComponentRotation` (`self.SM_Equipment_SwitchA`))) "Undefined" "MultiplyWithRoot" null null))
    (`StaticMeshComponent.SetStaticMesh` (`StaticMeshActor.StaticMeshComponent` _returnvalue) (`self.SwitchMesh`))
    (set `self.isPlaced` true)))

(fn `UserConstructionScript`
  (`StaticMeshComponent.SetStaticMesh` (`self.SM_Equipment_SwitchA`) (`self.SwitchMesh`)))